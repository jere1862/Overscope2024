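; BP_SharedCamera is a shared camera actor that tracks the midpoint of the player characters.
; Half a second after BeginPlay, it caches all BP_ThirdPersonCharacter actors and enables its tick.
; Each tick, UpdateCenterLocation averages their locations and moves the Billboard component to that center.
; The construction script rotates the Camera to look at the Root component.
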(event EventBeginPlay
  ;[0 0 0] Begin play
  (Utilities|FlowControl|Delay 0.5)
  (bind _outactors (Actor|GetAllActorsOfClass "/Game/ThirdPerson/Blueprints/BP_ThirdPersonCharacter.BP_ThirdPersonCharacter_C"))
  (Variables|Default|SetPawns _outactors)
  (Actor|Tick|SetActorTickEnabled true))

(event EventTick
  (params (DeltaSeconds :type Float%20%28single-precision%29))
  ;[0 0 0] TICK !
  (CallFunction|UpdateCenterLocation) ; Move camera center to the center of the two players
)

(fn ConstructionScript
  ;[1 1 1] Force rotate camera to the root (look at)
  (Transformation|SetRelativeRotation (Variables|Default|GetCamera) (Math|Rotator|MakeRotfromX (Math|Vector|Normalize (- (Transformation|GetWorldLocation (Variables|Default|GetRoot)) (Transformation|GetWorldLocation (Variables|Default|GetCamera))))) false false))

(fn UpdateCenterLocation
  (bind _pawns (Variables|Default|GetPawns))
  (for _array_element _pawns
    (LocalVariables|SetAddTransform (+ (LocalVariables|GetAddTransform) (Transformation|GetActorLocation _array_element))))
  (Transformation|SetWorldLocation (Variables|Default|GetBillboard) (/ (LocalVariables|GetAddTransform) (Utilities|Array|Length _pawns)) false false))