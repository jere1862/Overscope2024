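; BP_Boom is a short-lived billboard effect actor, apparently a boom or explosion visual.
; On BeginPlay it picks a random sprite from SpritesRef, pulls the billboard toward the first player's camera by a fixed offset, and randomizes its scale.
; After a brief random delay it sets a very short lifespan, so each instance removes itself at a slightly different time.
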(event EventBeginPlay
  (Rendering|Components|Sprite|SetSprite (Variables|Default|GetBillboard) (Utilities|Array|Get(acopy) (Variables|Default|GetSpritesRef) (Math|Random|RandomIntegerinRange 0 3)))
  (Transformation|SetWorldLocation (Variables|Default|GetBillboard) (+ (* (Math|Vector|Normalize (- (Camera|GetCameraLocation (Variables|/Script/Engine.PlayerController|GetPlayerCameraManager (Game|GetPlayerController 0))) (Transformation|GetActorLocation))) 2e+02) (Transformation|GetWorldLocation (Variables|Default|GetBillboard))) false false)
  (Transformation|SetRelativeScale3D (Variables|Default|GetBillboard) (* "1.000000,1.000000,1.000000" (Math|Random|RandomFloatinRange 0.65 1.2)))
  (Utilities|FlowControl|Delay (Math|Random|RandomFloatinRange 0.2 0.6))
  (Actor|SetLifeSpan 0.1))

(fn ConstructionScript)